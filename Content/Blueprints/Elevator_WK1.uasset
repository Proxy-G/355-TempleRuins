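; Elevator actor that carries the player up a procedurally built shaft, with openings on opposite sides at the bottom and top floors.
; The construction script stacks instanced wall meshes per floor and derives travel distance from MaxFloors.
; A timeline, rate-scaled by velocity over distance, drives the Moving component's height.
; The collider enables interact input while FirstPersonCharacterWK1 overlaps; Interact plays the timeline, and leaving reverses it.
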(event OnComponentEndOverlap(Collider)
  (params (OverlappedComponent :type Primitive%20Component%20Object%20Reference) (OtherActor :type Actor%20Object%20Reference) (OtherComp :type Primitive%20Component%20Object%20Reference) (OtherBodyIndex :type Integer))
  (Utilities|Casting|CastToFirstPersonCharacterWK1 OtherActor)
  (Input|DisableInput (Game|GetPlayerController 0))
  (bind _percent (Timeline|ElevatorMove Reverse)
    (:Update
      (Transformation|SetRelativeLocation (Variables|Default|GetMoving) (Math|Vector|MakeVector 0.0 0.0 (* _percent (Variables|Default|GetElevatorDistance))) false false))))

(event OnComponentBeginOverlap(Collider)
  (params (OverlappedComponent :type Primitive%20Component%20Object%20Reference) (OtherActor :type Actor%20Object%20Reference) (OtherComp :type Primitive%20Component%20Object%20Reference) (OtherBodyIndex :type Integer) (bFromSweep :type Boolean) (SweepResult :type Hit%20Result%20Structure%20%28by%20ref%29))
  (Utilities|Casting|CastToFirstPersonCharacterWK1 OtherActor)
  (Input|EnableInput (Game|GetPlayerController 0)))

(event EventPlayerWantstoInteract
  (params (Player%20%28Default%29 :type First%20Person%20Character%20Object%20Reference) (Player%20%28WK1%29 :type First%20Person%20Character%20WK1%20Object%20Reference))
  (bind _percent (Timeline|ElevatorMove Play)
    (:Update
      (Transformation|SetRelativeLocation (Variables|Default|GetMoving) (Math|Vector|MakeVector 0.0 0.0 (* _percent (Variables|Default|GetElevatorDistance))) false false))))

(event EventBeginPlay
  (Components|Timeline|SetPlayRate (Variables|Default|GetElevatorMove) (/ (Variables|Default|GetElevatorVelocity) (Variables|Default|GetElevatorDistance))))

(event Input|ActionEvents|InputActionInteract
  (params (Key :type Key%20Structure))
  (:Pressed
    (bind _percent (Timeline|ElevatorMove Play)
      (:Update
        (Transformation|SetRelativeLocation (Variables|Default|GetMoving) (Math|Vector|MakeVector 0.0 0.0 (* _percent (Variables|Default|GetElevatorDistance))) false false)))))

(fn ConstructionScript
  (for _index (range 0 (Variables|Default|GetMaxFloors))
    (bind _output_get (LocalVariables|SetCurrentFloor _index))
    (LocalVariables|SetCurrentZ (* _output_get 4e+02))
    (Variables|Default|SetElevatorDistance (* (Variables|Default|GetMaxFloors) 4e+02))
    ;[1 1 1] right wall
    (Components|InstancedStaticMesh|AddInstance (Variables|Default|GetWallInstanceMesh) (Math|Transform|MakeTransform (Math|Vector|MakeVector -2e+02 2.1e+02 (LocalVariables|GetCurrentZ)) "0, 0, 0" "1,1,1"))
    ;[1 1 1] left wall
    (Components|InstancedStaticMesh|AddInstance (Variables|Default|GetWallInstanceMesh) (Math|Transform|MakeTransform (Math|Vector|MakeVector -2e+02 -2.1e+02 (LocalVariables|GetCurrentZ)) "0, 0, 0" "1,1,1"))
    ;[1 1 1] back wall
    (if (!= (LocalVariables|GetCurrentFloor) (Variables|Default|GetMaxFloors))
      (Components|InstancedStaticMesh|AddInstance (Variables|Default|GetWallInstanceMesh) (Math|Transform|MakeTransform (Math|Vector|MakeVector 2.1e+02 -2e+02 (LocalVariables|GetCurrentZ)) "0,90.000000, 0" "1,1,1")))
    ;[1 1 1] front wall
    (if (!= (LocalVariables|GetCurrentFloor) 0)
      (Components|InstancedStaticMesh|AddInstance (Variables|Default|GetWallInstanceMesh) (Math|Transform|MakeTransform (Math|Vector|MakeVector -2.1e+02 -2e+02 (LocalVariables|GetCurrentZ)) "0,90.000000, 0" "1,1,1")))))