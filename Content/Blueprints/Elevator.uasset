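; Elevator actor that the first-person player raises with the Interact input while standing inside its trigger collider.
; Overlapping the collider enables input on the actor, and leaving it disables input and reverses the ElevatorMove timeline.
; The timeline sets the Moving component's relative Z from its percent times ElevatorDistance.
; BeginPlay derives the play rate from velocity over distance, so travel speed follows ElevatorVelocity.
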(event OnComponentEndOverlap(Collider)
  (params (OverlappedComponent :type Primitive%20Component%20Object%20Reference) (OtherActor :type Actor%20Object%20Reference) (OtherComp :type Primitive%20Component%20Object%20Reference) (OtherBodyIndex :type Integer))
  (Utilities|Casting|CastToFirstPersonCharacter OtherActor)
  (Input|DisableInput (Game|GetPlayerController 0))
  (bind _percent (Timeline|ElevatorMove Reverse)
    (:Update
      (Transformation|SetRelativeLocation (Variables|Default|GetMoving) (Math|Vector|MakeVector 0.0 0.0 (* _percent (Variables|Default|GetElevatorDistance))) false false))))

(event OnComponentBeginOverlap(Collider)
  (params (OverlappedComponent :type Primitive%20Component%20Object%20Reference) (OtherActor :type Actor%20Object%20Reference) (OtherComp :type Primitive%20Component%20Object%20Reference) (OtherBodyIndex :type Integer) (bFromSweep :type Boolean) (SweepResult :type Hit%20Result%20Structure%20%28by%20ref%29))
  (Utilities|Casting|CastToFirstPersonCharacter OtherActor)
  (Input|EnableInput (Game|GetPlayerController 0)))

(event EventBeginPlay
  (Components|Timeline|SetPlayRate (Variables|Default|GetElevatorMove) (/ (Variables|Default|GetElevatorVelocity) (Variables|Default|GetElevatorDistance))))

(event Input|ActionEvents|InputActionInteract
  (params (Key :type Key%20Structure :default "None"))
  (:Pressed
    (bind _percent (Timeline|ElevatorMove Play)
      (:Update
        (Transformation|SetRelativeLocation (Variables|Default|GetMoving) (Math|Vector|MakeVector 0.0 0.0 (* _percent (Variables|Default|GetElevatorDistance))) false false)))))

(fn ConstructionScript)