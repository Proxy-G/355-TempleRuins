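; Lever actor that a player toggles to trigger another linked actor.
; On interaction it sends an interface message to its controlled actor if that implements ToggleableObject, then flips its on state and target angle.
; Tick eases the lever pivot's pitch toward the target with a frame-time lerp, switching itself off once the rotation is nearly reached.
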(event EventTick
  (params (DeltaSeconds :type Float%20%28single-precision%29))
  ;[1 1 1] Rotate Level Based On Activation
  (Variables|Default|SetdeltaTime DeltaSeconds)
  (Transformation|SetRelativeRotation (Variables|Default|GetLeverPivot) (Math|Rotator|MakeRotator 0.0 (Math|Float|Lerp (.pitch (Variables|/Script/Engine.SceneComponent|GetRelativeRotation (Variables|Default|GetLeverPivot))) (Variables|Default|GettargetLeverRotation) (* (Variables|Default|GetdeltaTime) 4.0)) 0.0) false false)
  ;[1 1 1] Anims Done Check
  (Actor|Tick|SetActorTickEnabled (not (Math|Float|NearlyEqual(Float) (.pitch (Variables|/Script/Engine.SceneComponent|GetRelativeRotation (Variables|Default|GetLeverPivot))) (Variables|Default|GettargetLeverRotation) 1.0))))

(event EventPlayerWantstoInteract
  (params (Player :type First%20Person%20Character%20Object%20Reference))
  (bind _other_actors_controlled_by_this_actor (Variables|Default|GetOther%20Actors%20Controlled%20By%20This%20Actor))
  ;[1 1 1] Set Other Actor To Do Their Action If They Can
  (Utilities|IsValid _other_actors_controlled_by_this_actor
    (:Is%20Valid
      (if (Utilities|DoesObjectImplementInterface _other_actors_controlled_by_this_actor "/Game/Blueprints/ToggleableObject.ToggleableObject_C")
        (Class|ToggleableObject|Interact(Message) _other_actors_controlled_by_this_actor)
        (if (Variables|Default|GetisOn)
          (Variables|Default|SetisOn false)
          (Variables|Default|SettargetLeverRotation 0.0)
          (else
            (Variables|Default|SetisOn true)
            (Variables|Default|SettargetLeverRotation 9e+01)))
        (Actor|Tick|SetActorTickEnabled true)))))

(fn ConstructionScript)