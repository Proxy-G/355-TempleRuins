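; MyPlayerController is a player controller that owns the player's HUD widget.
; On BeginPlay it caches MyGameInstance, then creates the HUD and adds it to the viewport, doing nothing if the cast fails.
; Its UpdateHUD event passes the game instance's PlayerDetails to the widget, and Destroyed removes the widget from its parent.
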(event Custom|UpdateHUD
  (bind _hud (Variables|Default|GetHUD))
  (Utilities|IsValid _hud
    (:Is%20Valid
      (Default|UpdateHUD _hud (Variables|/Game/Blueprints/PlayerGame/MyGameInstance.MyGameInstance_C|GetplayerDetails (Variables|Default|GetGame%20Instance))))))

(event EventBeginPlay
  (bind _asmy_game_instance (Utilities|Casting|CastToMyGameInstance (Game|GetGameInstance)))
  (Variables|Default|SetGame%20Instance _asmy_game_instance)
  (bind _returnvalue (UserInterface|CreateWidget "/Game/Blueprints/GUI/HUD.HUD_C"))
  (bind _output_get (Variables|Default|SetHUD _returnvalue))
  (UserInterface|Viewport|AddtoViewport _output_get 0))

(event EventDestroyed
  (bind _hud (Variables|Default|GetHUD))
  (Utilities|IsValid _hud
    (:Is%20Valid
      (Widget|RemovefromParent _hud))))

(fn ConstructionScript)