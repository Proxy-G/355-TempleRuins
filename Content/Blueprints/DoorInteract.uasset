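; Interactive hinged door Blueprint that swings open and closed around a pivot when interacted with.
; Interact toggles the open state, sets a target yaw, plays an open or close sound and enables actor tick.
; Tick eases the pivot's yaw toward the target with a delta-time-scaled lerp, then disables ticking once nearly there, so it only ticks while moving.
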(event EventTurnOff
  (params (Player :type First%20Person%20Character%20Interface%20Object%20Reference))
  ;[1 1 1] Set The Door Rotation Upon Interaction
  (Variables|Default|SettargetDoorRotation 0.0)
  (Variables|Default|SetIsDoorOpen false)
  (Audio|PlaySoundatLocation (Variables|Default|GetdoorCloseSFX) (Transformation|GetActorLocation) "0, 0, 0" 1.0 1.0 0.0 0 0 0)
  (Actor|Tick|SetActorTickEnabled true))

(event EventTurnon
  (params (Player :type First%20Person%20Character%20Interface%20Object%20Reference))
  ;[1 1 1] Set The Door Rotation Upon Interaction
  (Variables|Default|SettargetDoorRotation 1e+02)
  (Variables|Default|SetIsDoorOpen true)
  (Audio|PlaySoundatLocation (Variables|Default|GetdoorOpenSFX) (Transformation|GetActorLocation) "0, 0, 0" 1.0 1.0 0.0 0 0 0)
  (Actor|Tick|SetActorTickEnabled true))

(event EventTick
  (params (DeltaSeconds :type Float%20%28single-precision%29))
  ;[1 1 1] Enable/Disable Input, Rotate Door To Target Door Rotation
  (Variables|Default|SetdeltaTime DeltaSeconds)
  (Transformation|SetRelativeRotation (Variables|Default|GetDoorTurnPivot) (Math|Rotator|MakeRotator 0.0 0.0 (Math|Float|Lerp (.yaw (Variables|/Script/Engine.SceneComponent|GetRelativeRotation (Variables|Default|GetDoorTurnPivot))) (Variables|Default|GettargetDoorRotation) (* (Variables|Default|GetdeltaTime) 4.0))) false false)
  ;[1 1 1] Anims Done Check
  (Actor|Tick|SetActorTickEnabled (not (Math|Float|NearlyEqual(Float) (.yaw (Variables|/Script/Engine.SceneComponent|GetRelativeRotation (Variables|Default|GetDoorTurnPivot))) (Variables|Default|GettargetDoorRotation) 1.0))))

(event EventInteract
  ;[1 1 1] Set The Door Rotation Upon Interaction
  (if (Variables|Default|GetIsDoorOpen)
    (CallFunction|TurnOff)
    (else
      (CallFunction|Turnon))))

(fn ConstructionScript)