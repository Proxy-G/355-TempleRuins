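; DroneBP is a player-controlled drone that flies forward, back, up and down, and turns in yaw.
; Movement axes feed movement input, while MoveRight sets a desired rotation velocity scaled by sensitivity.
; Tick eases the current yaw velocity toward that target and switches itself off when rotation is negligible, until new turn input re-enables it.
; Pressing Deploy repossesses the Player, sets its turn and look-up rates, and destroys the drone.
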(event EventTick
  (params (DeltaSeconds :type Float%20%28single-precision%29))
  ;[1 1 1] Smooth Rotate Drone
  (bind _output_get (Variables|Default|SetcurrentRotVelocity (Math|Float|Lerp (Variables|Default|GetcurrentRotVelocity) (Variables|Default|GetdesiredRotVelocity) (* DeltaSeconds 4.0))))
  (Transformation|AddActorLocalRotation (Math|Rotator|MakeRotator 0.0 0.0 _output_get) false false)
  (Actor|Tick|SetActorTickEnabled (> (Math|Float|Absolute(Float) (Variables|Default|GetcurrentRotVelocity)) 0.05)))

(event Input|ActionEvents|InputActionDeploy
  (params (Key :type Key%20Structure))
  (bind _player (Variables|Default|Getplayer))
  ;[1 1 1] Exit Drone
  (:Pressed
    (Pawn|Possess (Pawn|GetController) _player)
    (Variables|/Game/Blueprints/PlayerGame/FirstPersonCharacter.FirstPersonCharacter_C|SetBaseTurnRate _player 45.0)
    (Variables|/Game/Blueprints/PlayerGame/FirstPersonCharacter.FirstPersonCharacter_C|SetBaseLookUpRate _player 45.0)
    (Actor|DestroyActor)))

(event Input|AxisEvents|InputAxisMoveUpDown
  (params (AxisValue :type Float%20%28single-precision%29))
  ;[1 1 1] Forward/Backward Movement
  (Pawn|Input|AddMovementInput (Transformation|GetActorUpVector) AxisValue false))

(event Input|AxisEvents|InputAxisMoveForward
  (params (AxisValue :type Float%20%28single-precision%29))
  ;[1 1 1] Forward/Backward Movement
  (Pawn|Input|AddMovementInput (Transformation|GetActorForwardVector) AxisValue false))

(event Input|AxisEvents|InputAxisMoveRight
  (params (AxisValue :type Float%20%28single-precision%29))
  ;[1 1 1] Set Drone Rotate Velocity
  (bind _output_get (Variables|Default|SetdesiredRotVelocity (* AxisValue (Variables|Default|GetrotateSensitivity))))
  (if (> (Math|Float|Absolute(Float) _output_get) 0.05)
    (Actor|Tick|SetActorTickEnabled true)))

(fn ConstructionScript)