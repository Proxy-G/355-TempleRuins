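; Interactable elevator that toggles between rising and descending whenever it receives a Trigger or Interact event.
; Its construction script builds the shaft from instanced wall meshes per floor, leaving front open at bottom and back open at top, and derives travel distance from floor count.
; A timeline plays or reverses to drive the moving component's height, with play rate scaled by velocity over distance to keep speed independent of height.
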(event EventTrigger
  ;[1 1 1] Toggle On/Off
  (if (Variables|Default|GetisOn)
    (Variables|Default|SetisOn false)
    (CallFunction|TurnOff)
    (else
      (Variables|Default|SetisOn true)
      (CallFunction|Turnon))))

(event EventTurnon
  (params (Player :type First%20Person%20Character%20Object%20Reference))
  ;[1 1 1] Control Elevator
  (bind _percent (Timeline|ElevatorMove Play)
    (:Update
      (Transformation|SetRelativeLocation (Variables|Default|GetMoving) (Math|Vector|MakeVector 0.0 0.0 (* _percent (Variables|Default|GetElevatorDistance))) false false))))

(event EventTurnOff
  (params (Player :type First%20Person%20Character%20Object%20Reference))
  ;[1 1 1] Control Elevator
  (bind _percent (Timeline|ElevatorMove Reverse)
    (:Update
      (Transformation|SetRelativeLocation (Variables|Default|GetMoving) (Math|Vector|MakeVector 0.0 0.0 (* _percent (Variables|Default|GetElevatorDistance))) false false))))

(event EventInteract
  ;[1 1 1] Toggle On/Off
  (if (Variables|Default|GetisOn)
    (Variables|Default|SetisOn false)
    (CallFunction|TurnOff)
    (else
      (Variables|Default|SetisOn true)
      (CallFunction|Turnon))))

(event EventBeginPlay
  ;[1 1 1] Set Elevator Rise Rate
  (Components|Timeline|SetPlayRate (Variables|Default|GetElevatorMove) (/ (Variables|Default|GetElevatorVelocity) (Variables|Default|GetElevatorDistance))))

(fn ConstructionScript
  (for _index (range 0 (Variables|Default|GetMaxFloors))
    (bind _output_get (LocalVariables|SetCurrentFloor _index))
    (LocalVariables|SetCurrentZ (* _output_get 4e+02))
    (Variables|Default|SetElevatorDistance (* (Variables|Default|GetMaxFloors) 4e+02))
    ;[1 1 1] right wall
    (Components|InstancedStaticMesh|AddInstance (Variables|Default|GetWallInstanceMesh) (Math|Transform|MakeTransform (Math|Vector|MakeVector -2e+02 2.1e+02 (LocalVariables|GetCurrentZ)) "0, 0, 0" "1,1,1"))
    ;[1 1 1] left wall
    (Components|InstancedStaticMesh|AddInstance (Variables|Default|GetWallInstanceMesh) (Math|Transform|MakeTransform (Math|Vector|MakeVector -2e+02 -2.1e+02 (LocalVariables|GetCurrentZ)) "0, 0, 0" "1,1,1"))
    ;[1 1 1] back wall
    (if (!= (LocalVariables|GetCurrentFloor) (Variables|Default|GetMaxFloors))
      (Components|InstancedStaticMesh|AddInstance (Variables|Default|GetWallInstanceMesh) (Math|Transform|MakeTransform (Math|Vector|MakeVector 2.1e+02 -2e+02 (LocalVariables|GetCurrentZ)) "0,90.000000, 0" "1,1,1")))
    ;[1 1 1] front wall
    (if (!= (LocalVariables|GetCurrentFloor) 0)
      (Components|InstancedStaticMesh|AddInstance (Variables|Default|GetWallInstanceMesh) (Math|Transform|MakeTransform (Math|Vector|MakeVector -2.1e+02 -2e+02 (LocalVariables|GetCurrentZ)) "0,90.000000, 0" "1,1,1")))))