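; Interactive door Blueprint that the first-person character opens away or closes with the Interact input, with sounds and a locked-door response.
; Front and back overlap volumes gate input and choose swing direction, while a third volume blocks closing.
; Tick lerps the pivot's yaw toward a target and switches itself off once close.
; The locked jiggle flips that target on successive ticks, as its tolerance checks never read the actual yaw.
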(event OnComponentBeginOverlap(ColliderF)
  (params (OverlappedComponent :type Primitive%20Component%20Object%20Reference) (OtherActor :type Actor%20Object%20Reference) (OtherComp :type Primitive%20Component%20Object%20Reference) (OtherBodyIndex :type Integer) (bFromSweep :type Boolean) (SweepResult :type Hit%20Result%20Structure%20%28by%20ref%29))
  ;[1 1 1] Detect Player In Front Collider
  (Utilities|Casting|CastToFirstPersonCharacterDoor OtherActor)
  (Variables|Default|SetInColliderF true)
  (if (and (Variables|Default|GetnoAnim) (or (Variables|Default|GetInColliderF) (Variables|Default|GetInColliderB)))
    (Input|EnableInput (Game|GetPlayerController 0))
    (else
      (Input|DisableInput (Game|GetPlayerController 0)))))

(event OnComponentBeginOverlap(ColliderB)
  (params (OverlappedComponent :type Primitive%20Component%20Object%20Reference) (OtherActor :type Actor%20Object%20Reference) (OtherComp :type Primitive%20Component%20Object%20Reference) (OtherBodyIndex :type Integer) (bFromSweep :type Boolean) (SweepResult :type Hit%20Result%20Structure%20%28by%20ref%29))
  ;[1 1 1] Detect Player In BackCollider
  (Utilities|Casting|CastToFirstPersonCharacterDoor OtherActor)
  (Variables|Default|SetInColliderB true)
  (if (and (Variables|Default|GetnoAnim) (or (Variables|Default|GetInColliderF) (Variables|Default|GetInColliderB)))
    (Input|EnableInput (Game|GetPlayerController 0))
    (else
      (Input|DisableInput (Game|GetPlayerController 0)))))

(event OnComponentEndOverlap(ColliderB)
  (params (OverlappedComponent :type Primitive%20Component%20Object%20Reference) (OtherActor :type Actor%20Object%20Reference) (OtherComp :type Primitive%20Component%20Object%20Reference) (OtherBodyIndex :type Integer))
  ;[1 1 1] Detect Player In BackCollider
  (Utilities|Casting|CastToFirstPersonCharacterDoor OtherActor)
  (Variables|Default|SetInColliderB false)
  (if (and (Variables|Default|GetnoAnim) (or (Variables|Default|GetInColliderF) (Variables|Default|GetInColliderB)))
    (Input|EnableInput (Game|GetPlayerController 0))
    (else
      (Input|DisableInput (Game|GetPlayerController 0)))))

(event OnComponentEndOverlap(ColliderF)
  (params (OverlappedComponent :type Primitive%20Component%20Object%20Reference) (OtherActor :type Actor%20Object%20Reference) (OtherComp :type Primitive%20Component%20Object%20Reference) (OtherBodyIndex :type Integer))
  ;[1 1 1] Detect Player In Front Collider
  (Utilities|Casting|CastToFirstPersonCharacterDoor OtherActor)
  (Variables|Default|SetInColliderF false)
  (if (and (Variables|Default|GetnoAnim) (or (Variables|Default|GetInColliderF) (Variables|Default|GetInColliderB)))
    (Input|EnableInput (Game|GetPlayerController 0))
    (else
      (Input|DisableInput (Game|GetPlayerController 0)))))

(event OnComponentBeginOverlap(PreventCloseCollider)
  (params (OverlappedComponent :type Primitive%20Component%20Object%20Reference) (OtherActor :type Actor%20Object%20Reference) (OtherComp :type Primitive%20Component%20Object%20Reference) (OtherBodyIndex :type Integer) (bFromSweep :type Boolean) (SweepResult :type Hit%20Result%20Structure%20%28by%20ref%29))
  ;[1 1 1] Detect Player In Prevent Collider
  (Utilities|Casting|CastToFirstPersonCharacterDoor OtherActor)
  (Variables|Default|SetinPreventCollider true))

(event OnComponentEndOverlap(PreventCloseCollider)
  (params (OverlappedComponent :type Primitive%20Component%20Object%20Reference) (OtherActor :type Actor%20Object%20Reference) (OtherComp :type Primitive%20Component%20Object%20Reference) (OtherBodyIndex :type Integer))
  ;[1 1 1] Detect Player In Prevent Collider
  (Utilities|Casting|CastToFirstPersonCharacterDoor OtherActor)
  (Variables|Default|SetinPreventCollider false))

(event EventTick
  (params (DeltaSeconds :type Float%20%28single-precision%29))
  ;[1 1 1] Enable/Disable Input, Rotate Door To Target Door Rotation
  (Variables|Default|SetdeltaTime DeltaSeconds)
  (Transformation|SetRelativeRotation (Variables|Default|GetDoorTurnPivot) (Math|Rotator|MakeRotator 0.0 0.0 (Math|Float|Lerp (.yaw (Variables|/Script/Engine.SceneComponent|GetRelativeRotation (Variables|Default|GetDoorTurnPivot))) (Variables|Default|GettargetDoorRotation) (* (Variables|Default|GetdeltaTime) 4.0))) false false)
  ;[1 1 1] Door Locked Anim Logic
  (if (Variables|Default|GetdoorLockAnim)
    (if (== (Variables|Default|GettargetDoorRotation) 6.0)
      (if (Math|Float|NearlyEqual(Float) 6.0 (Variables|Default|GettargetDoorRotation) 0.1)
        (Variables|Default|SettargetDoorRotation -6.0))
      (elif (== (Variables|Default|GettargetDoorRotation) -6.0)
        (if (Math|Float|NearlyEqual(Float) -6.0 (Variables|Default|GettargetDoorRotation) 0.1)
          (Variables|Default|SettargetDoorRotation 0.0))
        (elif (== (Variables|Default|GettargetDoorRotation) 0.0)
          (if (Math|Float|NearlyEqual(Float) 0.0 0.0 0.1)
            (Variables|Default|SetdoorLockAnim false)
            (Variables|Default|SetnoAnim false)))))
    (else
      ;[1 1 1] Anims Done Check
      (Variables|Default|SetnoAnim (Math|Float|NearlyEqual(Float) (.yaw (Variables|/Script/Engine.SceneComponent|GetRelativeRotation (Variables|Default|GetDoorTurnPivot))) (Variables|Default|GettargetDoorRotation) 2.5))
      (Actor|Tick|SetActorTickEnabled (not (Math|Float|NearlyEqual(Float) (.yaw (Variables|/Script/Engine.SceneComponent|GetRelativeRotation (Variables|Default|GetDoorTurnPivot))) (Variables|Default|GettargetDoorRotation) 2.5))))))

(event Input|ActionEvents|InputActionInteract
  (params (Key :type Key%20Structure :default "None"))
  (bind _returnvalue (Transformation|GetActorLocation))
  ;[1 1 1] Set The Door Rotation Upon Interaction
  (:Pressed
    (if (Variables|Default|GetIsDoorOpen)
      (if (not (Variables|Default|GetinPreventCollider))
        (Variables|Default|SettargetDoorRotation 0.0)
        (Variables|Default|SetIsDoorOpen false)
        (Audio|PlaySoundatLocation (Variables|Default|GetdoorCloseSFX) _returnvalue "0, 0, 0" 1.0 1.0 0.0 0 0 0)
        (Variables|Default|SetnoAnim true :!label _label)
        (Actor|Tick|SetActorTickEnabled true))
      (elif (Variables|Default|GetIsDoorLocked)
        (Variables|Default|SettargetDoorRotation 6.0)
        (Variables|Default|SetdoorLockAnim true)
        (Development|PrintString "Door must be locked...")
        (Audio|PlaySoundatLocation (Variables|Default|GetdoorLockedSFX) _returnvalue "0, 0, 0" 1.0 1.0 0.0 0 0 0)
        (goto _label)
        (else
          (if (Variables|Default|GetInColliderF)
            (Variables|Default|SettargetDoorRotation 1e+02)
            (Variables|Default|SetIsDoorOpen true)
            (else
              (Variables|Default|SettargetDoorRotation -75.0)
              (Variables|Default|SetIsDoorOpen true)))
          (Audio|PlaySoundatLocation (Variables|Default|GetdoorOpenSFX) _returnvalue "0, 0, 0" 1.0 1.0 0.0 0 0 0)
          (goto _label))))))

(fn ConstructionScript)