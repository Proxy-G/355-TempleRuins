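; Button actor that toggles a linked actor when a FirstPersonCharacterInterface character enters or leaves its collision.
; Overlap events check that the linked actor implements ToggleableObject, set the on/off state, restart a short countdown and enable Tick.
; Tick debounces the input: once the countdown expires, it sends InteractMessage only if the state differs from the previous one, then disables itself.
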(event OnComponentBeginOverlap(ButtonCollision)
  (params (OverlappedComponent :type Primitive%20Component%20Object%20Reference) (OtherActor :type Actor%20Object%20Reference) (OtherComp :type Primitive%20Component%20Object%20Reference) (OtherBodyIndex :type Integer) (bFromSweep :type Boolean) (SweepResult :type Hit%20Result%20Structure%20%28by%20ref%29))
  (bind _other_actors_controlled_by_this_actor (Variables|Default|GetOther%20Actors%20Controlled%20By%20This%20Actor))
  ;[1 1 1] Detect Player In Front Collider
  (Utilities|Casting|CastToFirstPersonCharacterInterface OtherActor)
  (Utilities|IsValid _other_actors_controlled_by_this_actor
    (:Is%20Valid
      (if (Utilities|DoesObjectImplementInterface _other_actors_controlled_by_this_actor "/Game/Blueprints/ToggleableObject.ToggleableObject_C")
        (Variables|Default|SetisOn true)
        (Variables|Default|SettimeWait 0.1)
        (Actor|Tick|SetActorTickEnabled true)))))

(event OnComponentEndOverlap(ButtonCollision)
  (params (OverlappedComponent :type Primitive%20Component%20Object%20Reference) (OtherActor :type Actor%20Object%20Reference) (OtherComp :type Primitive%20Component%20Object%20Reference) (OtherBodyIndex :type Integer))
  (bind _other_actors_controlled_by_this_actor (Variables|Default|GetOther%20Actors%20Controlled%20By%20This%20Actor))
  ;[1 1 1] Detect Player In Front Collider
  (Utilities|Casting|CastToFirstPersonCharacterInterface OtherActor)
  (Utilities|IsValid _other_actors_controlled_by_this_actor
    (:Is%20Valid
      (if (Utilities|DoesObjectImplementInterface _other_actors_controlled_by_this_actor "/Game/Blueprints/ToggleableObject.ToggleableObject_C")
        (Variables|Default|SetisOn false)
        (Variables|Default|SettimeWait 0.1)
        (Actor|Tick|SetActorTickEnabled true)))))

(event EventTick
  (params (DeltaSeconds :type Float%20%28single-precision%29))
  ;[1 1 1] Button Check State
  (bind _output_get (Variables|Default|SetdeltaTime DeltaSeconds))
  (Variables|Default|SettimeWait (- (Variables|Default|GettimeWait) _output_get))
  (if (<= (- (Variables|Default|GettimeWait) _output_get) 0.0)
    (if (Math|Boolean|NotEqual(Boolean) (Variables|Default|GetisOn) (Variables|Default|GetisOnPrev))
      (Class|ToggleableObject|Interact(Message) (Variables|Default|GetOther%20Actors%20Controlled%20By%20This%20Actor))
      (Variables|Default|SetisOnPrev (Variables|Default|GetisOn))
      (Actor|Tick|SetActorTickEnabled false))))

(fn ConstructionScript)